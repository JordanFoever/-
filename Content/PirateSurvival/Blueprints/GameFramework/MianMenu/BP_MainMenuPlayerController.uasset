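; Player controller for the main menu that shows the menu widget and switches camera views.
; On BeginPlay it adds WBP_MainMenu to the viewport and sets the view target to the MainCamera of the possessed BP_MainMenuDummyPawn.
; NewGameOperate calls NewGame, which blends the view over to that pawn's CharacterCamera.
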(event EventBeginPlay
  (bind _returnvalue (UserInterface|CreateWidget "/Game/PirateSurvival/UI/MainMenu/WBP_MainMenu.WBP_MainMenu_C"))
  (UserInterface|Viewport|AddtoViewport _returnvalue 0)
  (bind _asbp_main_menu_dummy_pawn (Utilities|Casting|CastToBP_MainMenuDummyPawn (Pawn|GetControlledPawn)))
  (Game|Player|SetViewTargetwithBlend (Variables|/Game/PirateSurvival/Blueprints/GameFramework/MianMenu/BP_MainMenuDummyPawn.BP_MainMenuDummyPawn_C|GetMainCamera _asbp_main_menu_dummy_pawn) 0.0 "VTBlend_Linear" 0.0 false))

(event EventNewGameOperate
  (CallFunction|NewGame))

(fn ConstructionScript)

(fn NewGame
  (bind _asbp_main_menu_dummy_pawn (Utilities|Casting|CastToBP_MainMenuDummyPawn (Pawn|GetControlledPawn)))
  (Game|Player|SetViewTargetwithBlend (Variables|/Game/PirateSurvival/Blueprints/GameFramework/MianMenu/BP_MainMenuDummyPawn.BP_MainMenuDummyPawn_C|GetCharacterCamera _asbp_main_menu_dummy_pawn) 2.0 "VTBlend_Linear" 0.0 false))