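; Door building part for the pirate survival building system that swings open and closed when interacted with.
; The first interaction caches a hinge pivot and arm vector from two mesh sockets, plus the actor's rotation.
; Each interaction moves and rotates the mesh by the stored yaw, then sets the next angle, with debug output.
; A separate helper adds destructible components that ignore Pawn and Camera collision.
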(event EventInteractiveResponse
  (params (Controller :type Player%20Controller%20Object%20Reference))
  (bind _buildingpartmesh (Variables|Default|GetBuildingPartMesh))
  (bind _buildingpartmesh_2 (Variables|Default|GetBuildingPartMesh))
  (bind _returnvalue (Transformation|GetSocketLocation _buildingpartmesh "Socket"))
  (Development|PrintString "Door")
  (Utilities|FlowControl|Sequence
    (:then_0
      (Utilities|FlowControl|DoOnce false
        (:Completed
          (Variables|Default|SetRotatePivot _returnvalue)
          (Variables|Default|SetRotateVector (- (Transformation|GetSocketLocation _buildingpartmesh "Socket1") _returnvalue))
          (Variables|Default|SetOriginRotation (Transformation|GetActorRotation)))))
    (:then_1
      (Utilities|FlowControl|Sequence
        (:then_0
          (Variables|Default|SetIsDoorOpened (not (Variables|Default|GetIsDoorOpened)))
          (Transformation|SetWorldLocation _buildingpartmesh_2 (+ (Math|Vector|RotateVectorAroundAxis (Variables|Default|GetRotateVector) (Variables|Default|GetAngle) "0.000000, 0,1.000000") (Variables|Default|GetRotatePivot)) false false)
          (Transformation|SetWorldRotation _buildingpartmesh_2 (Math|Rotator|CombineRotators (Variables|Default|GetOriginRotation) (Math|Rotator|MakeRotator 0.0 0.0 (Variables|Default|GetAngle))) false false))
        (:then_1
          (if (Variables|Default|GetIsDoorOpened)
            (Variables|Default|SetAngle 0.0)
            (else
              (Variables|Default|SetAngle -9e+01))))
        (:then_2
          (Rendering|Debug|DrawDebugLine (Variables|Default|GetRotatePivot) (+ (Math|Vector|RotateVectorAroundAxis (Variables|Default|GetRotateVector) (Variables|Default|GetAngle) "0.000000, 0,1.000000") (Variables|Default|GetRotatePivot)) "(R=0.000000,G=0.368750,B=1.000000,A=1.000000)" 5.0 5.0))))))

(fn ConstructionScript)

(fn AddDestructibleComptoActor
  (params (Actor :type Actor%20Object%20Reference) (InTransform :type Transform))
  (bind _returnvalue (AddComponent|AddDestructibleComponent Actor false InTransform))
  (Collision|SetCollisionResponsetoChannel _returnvalue "ECC_Pawn" "ECR_Ignore")
  (Collision|SetCollisionResponsetoChannel _returnvalue "ECC_Camera" "ECR_Ignore")
  (return _returnvalue))