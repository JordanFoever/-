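; BP_BuildingPartActor is an actor for a piece in the building system, apparently left mostly as a stub.
; Its interaction response only prints a debug string, while Tick, construction and the misspelled destroy event are empty.
; Disconnected logic would swap the mesh for a short-lived, physics-simulated destructible actor that ignores Pawn and Camera, and scan overlapping components.
; A helper function adds a destructible component to a given actor.
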(event EventDestoryBuidlingPart)

(event EventInteractiveResponse
  (params (Controller :type Player%20Controller%20Object%20Reference))
  (Development|PrintString "BuildingPart"))

(event EventTick
  (params (DeltaSeconds :type Float%20%28single-precision%29)))

(fn ConstructionScript)

(fn AddDestructibleComptoActor
  (params (Actor :type Actor%20Object%20Reference) (InTransform :type Transform))
  (bind _returnvalue (AddComponent|AddDestructibleComponent Actor false InTransform))
  (return _returnvalue))