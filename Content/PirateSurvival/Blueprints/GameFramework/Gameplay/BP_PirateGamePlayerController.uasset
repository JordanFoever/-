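; Player controller for the pirate survival game that owns the game HUD, NPC dialogue and a simple quest list.
; On possess it creates the HUD and dialogue widgets and binds tagged delegates that move items from loot boxes into the inventory and from inventory to the hotbar.
; Tab and U toggle the HUD and save-confirm panel with input locking.
; Dialogue walks an index-linked graph, showing numbered choices at branches.
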(event EventQuest
  (params (Quest :type BP%20Quset%20Object%20Reference))
  (Utilities|Array|Add (Variables|Talk|GetQuests) Quest))

(event EventPossess
  (params (PossessedPawn :type Pawn%20Object%20Reference))
  (CallFunction|InitiatePossessed PossessedPawn)
  (Utilities|FlowControl|Sequence
    (:then_0
      (bind _returnvalue (UserInterface|CreateWidget "/Game/PirateSurvival/UI/Game/WBP_GameHUD.WBP_GameHUD_C"))
      (bind _output_get (Variables|Default|SetGameHUD _returnvalue))
      (UserInterface|Viewport|AddtoViewport _output_get 0)
      (Class|BPIPlayerInitiateMessageReceiver|OnGameUIInitiated(Message) PossessedPawn))
    (:then_1
      (bind _returnvalue_2 (UserInterface|CreateWidget "/Game/GameplayDemo/Blueprints/UI/WBP_DialogPannel.WBP_DialogPannel_C"))
      (bind _output_get_2 (Variables|Talk|SetWedgetDialog _returnvalue_2))
      (UserInterface|Viewport|AddtoViewport _output_get_2 0)
      (Widget|SetVisibility (Variables|Talk|GetWedgetDialog) "Collapsed"))))

(event EventHandleDialogSelected
  (params (Index :type Integer))
  (Default|ReplyDialog (Variables|Talk|GetCurrentDialogNPC) (Variables|Talk|GetDialogIndex) Index)
  (Variables|Talk|SetDialogIndex (Utilities|Array|Get(acopy) (.craphchild (Utilities|Array|Get(acopy) (.dialogcontent (Variables|Talk|GetCurrentDialog)) (Variables|Talk|GetDialogIndex))) Index))
  (Talk|ProssessDialog))

(event EventListenDialog
  (params (DialogContent :type Dialog%20Structure%20Structure))
  (Variables|Talk|SetCurrentDialog DialogContent)
  (Widget|SetVisibility (Variables|Talk|GetWedgetDialog) "Visible")
  (Input|SetInputModeGameandUI self (Variables|Talk|GetWedgetDialog) "DoNotLock" true)
  (Variables|Default|SetbShowMouseCursor true)
  (Class|GameplayStatics|SetViewportMouseCaptureMode "NoCapture")
  (Variables|Talk|SetProssessingDialog true)
  (Variables|Talk|SetCurrentDialogNPC (.AsBP%20NPC (Utilities|Casting|CastToBP_NPC (Variables|Default|GetInteractiveActor))))
  (Talk|ProssessDialog))

(event EventContinueDialog
  (Talk|ProssessDialog))

(event EventFinishDialogGraph
  (Talk|HandleFinishDialogGraph))

(event Input|KeyboardEvents|Tab
  (params (Key :type Key%20Structure :default "None"))
  (:Pressed
    (CallFunction|SetOpenGameHUD (not (Variables|Default|GetIsShowUI)))))

(event Input|KeyboardEvents|U
  (params (Key :type Key%20Structure :default "None"))
  (:Pressed
    (CallFunction|SetOpenSaveConfirmUI (not (Variables|Default|GetIsShowSaveConfirmUI)))))

(fn ConstructionScript)

(fn SetOpenGameHUD
  (params (Open :type Boolean))
  (bind _self self)
  (bind _output_get (Variables|Default|SetIsShowUI Open))
  (Default|ToggleShowGameUI (Variables|Default|GetGameHUD) _output_get)
  (bind _output_get_2 (Variables|Default|SetbShowMouseCursor (Variables|Default|GetIsShowUI)))
  (if _output_get_2
    ;[1 1 1] 停止人物的视角
    (Input|SetIgnoreLookInput true)
    ;[1 1 1] 停止人物的移动
    (Input|SetIgnoreMoveInput true)
    (Input|SetInputModeGameandUI _self (Variables|Default|GetGameHUD) "DoNotLock" false)
    (else
      (Input|ResetIgnoreLookInput)
      (Input|ResetIgnoreMoveInput)
      (Input|SetInputModeGameOnly _self))))

(fn InitiatePossessed
  (params (Possessed%20Pawn :type Pawn%20Object%20Reference))
  (bind _returnvalue (Class|AssociatedComponentGetter|GetDelegateComponent(Message) Possessed%20Pawn))
  (Utilities|IsValid _returnvalue
    (:Is%20Valid
      (Class|DelegateComponent|BindDelegate _returnvalue "(TagName=\"GlobalEvent.Interactive.LootItemBox\")" self "HandleLootItemBox") ; 调用委托在WBP_LootItemBox中的OnItemSlotRightDown(WBP_ITemSlotBox中)
      ;[1 1 1] 调用委托在WBP_PlayerInventory中
      (Class|DelegateComponent|BindDelegate _returnvalue "(TagName=\"GlobalEvent.PlayerInventory.AssignItemToHotBar\")" self "HandleAssignItemToHotBar"))))

(fn HandleLootItemBox
  (params (Payload :type Object%20Object%20Reference))
  (bind _asbp_player_inventory_drag_drop_payload (Utilities|Casting|CastToBP_PlayerInventoryDragDropPayload Payload)) ; 我懒得去声明了,直接偷懒用之前的
  (Utilities|FlowControl|Sequence
    (:then_0
      (bind _returnvalue (Class|AssociatedComponentGetter|GetInventoryComponent(Message) (Variables|Default|GetInteractiveActor)))
      (Utilities|IsValid _returnvalue
        (:Is%20Valid
          (LocalVariables|SetData (.OutData (Class|InventoryComponent|GetItemData _returnvalue (Variables|/Game/PirateSurvival/Blueprints/DelegatePayload/BP_PlayerInventoryDragDropPayload.BP_PlayerInventoryDragDropPayload_C|GetFrom _asbp_player_inventory_drag_drop_payload)))))))
    (:then_1
      (bind _returnvalue_2 (Class|AssociatedComponentGetter|GetInventoryComponent(Message) (Pawn|GetControlledPawn)))
      (Utilities|IsValid _returnvalue_2
        (:Is%20Valid
          (bind _returnvalue_3 (Class|InventoryComponent|AddItemtoInventory _returnvalue_2 (.tablerowname (LocalVariables|GetData)) (.count (LocalVariables|GetData)) 0 0 false))
          (Class|InventoryComponent|RemoveIndexfromInventory _returnvalue (Variables|/Game/PirateSurvival/Blueprints/DelegatePayload/BP_PlayerInventoryDragDropPayload.BP_PlayerInventoryDragDropPayload_C|GetFrom _asbp_player_inventory_drag_drop_payload) (- (.count (LocalVariables|GetData)) _returnvalue_3)))))))

(fn HandleAssignItemtoHotBar
  (params (Payload :type Object%20Object%20Reference))
  (bind _asbp_inventory_index_payload (Utilities|Casting|CastToBP_InventoryIndexPayload Payload))
  (LocalVariables|SetIndex (Variables|/Game/PirateSurvival/Blueprints/DelegatePayload/BP_InventoryIndexPayload.BP_InventoryIndexPayload_C|GetIndex _asbp_inventory_index_payload))
  (Utilities|FlowControl|Sequence
    (:then_0
      (bind _returnvalue (Class|AssociatedComponentGetter|GetInventoryComponent(Message) (Pawn|GetControlledPawn)))
      (LocalVariables|SetInventory _returnvalue)
      (bind _returnvalue_2 (Class|AssociatedComponentGetter|GetHotBarComponent(Message) (Pawn|GetControlledPawn)))
      (LocalVariables|SetHotBar _returnvalue_2)
      (if (not (and (Utilities|IsValid (LocalVariables|GetInventory)) (Utilities|IsValid (LocalVariables|GetHotBar))))
        (return)))
    (:then_1
      (if (.ReturnValue (Class|InventoryComponent|GetItemData (LocalVariables|GetInventory) (LocalVariables|GetIndex)))
        (bind _returnvalue_3 (Class|InventoryComponent|AddItemtoInventory (LocalVariables|GetHotBar) (.TableRowName (Utilities|Struct|BreakInventoryItemData (.OutData (Class|InventoryComponent|GetItemData (LocalVariables|GetInventory) (LocalVariables|GetIndex))))) (.Count (Utilities|Struct|BreakInventoryItemData (.OutData (Class|InventoryComponent|GetItemData (LocalVariables|GetInventory) (LocalVariables|GetIndex))))) 0 0 false))
        (if (== _returnvalue_3 0)
          (Class|InventoryComponent|RemoveIndexfromInventory (LocalVariables|GetInventory) (LocalVariables|GetIndex) (.Count (Utilities|Struct|BreakInventoryItemData (.OutData (Class|InventoryComponent|GetItemData (LocalVariables|GetInventory) (LocalVariables|GetIndex)))))))))))

(fn SetOpenSaveConfirmUI
  (params (Open :type Boolean))
  (bind _self self)
  (bind _output_get (Variables|Default|SetIsShowSaveConfirmUI Open))
  (Default|ToggleShowSaveConfirmPanel (Variables|Default|GetGameHUD) _output_get)
  (bind _output_get_2 (Variables|Default|SetbShowMouseCursor (Variables|Default|GetIsShowSaveConfirmUI)))
  (if _output_get_2
    (Input|SetIgnoreLookInput true)
    (Input|SetIgnoreMoveInput true)
    (Input|SetInputModeGameandUI _self (Variables|Default|GetGameHUD) "DoNotLock" true)
    (else
      (Input|SetIgnoreLookInput false)
      (Input|SetIgnoreMoveInput false)
      (Input|SetInputModeGameOnly _self))))

(fn ProssessDialog
  ;[1 1 1] 如果继续进行对话就获取这个对话中的一段从第一段开始并将这对话的内容 传给  add dialog Draph（DialogGraphStructure[ ]   DialogGraph）
  (if (Variables|Talk|GetProssessingDialog)
    (if (Utilities|Array|IsValidIndex (.dialogcontent (Variables|Talk|GetCurrentDialog)) (Variables|Talk|GetDialogIndex))
      (Default|AddDialogGraph (Variables|Talk|GetWedgetDialog) (.graph (Utilities|Array|Get(acopy) (.dialogcontent (Variables|Talk|GetCurrentDialog)) (Variables|Talk|GetDialogIndex)))))
    (else
      ;[1 1 1] 这个是结束对话时调用
      (Input|SetInputModeGameOnly self)
      (Variables|Default|SetbShowMouseCursor false)
      (Widget|SetVisibility (Variables|Talk|GetWedgetDialog) "Collapsed")
      (Class|GameplayStatics|SetViewportMouseCaptureMode "CapturePermanently") ; 永久捕获鼠标
      (Widget|Panel|ClearChildren (Variables|/Game/GameplayDemo/Blueprints/UI/WBP_DialogPannel.WBP_DialogPannel_C|GetScrollBox_DialogContainer (Variables|Talk|GetWedgetDialog))))))

(fn EndDialog
  (Variables|Talk|SetProssessingDialog false)
  (Default|AddEndDialogTip (Variables|Talk|GetWedgetDialog))
  (Variables|Talk|SetCurrentDialogNPC 0)
  (Variables|Talk|SetDialogIndex 0))

(fn HandleFinishDialogGraph
  (if (> (Utilities|Array|Length (.craphchild (Utilities|Array|Get(acopy) (.dialogcontent (Variables|Talk|GetCurrentDialog)) (Variables|Talk|GetDialogIndex)))) 1) ; 为true右分支，反之没有继续执行对话
    (for (_array_element _array_index) (.craphchild (Utilities|Array|Get(acopy) (.dialogcontent (Variables|Talk|GetCurrentDialog)) (Variables|Talk|GetDialogIndex)))
      (LocalVariables|SetSelectionString (Utilities|String|Append (Utilities|String|ToString(Integer) (+ _array_index 1)) ". "))
      (for _array_element_2 (.graph (Utilities|Array|Get(acopy) (.dialogcontent (Variables|Talk|GetCurrentDialog)) _array_element))
        (if (Utilities|Enum|Equal(Enum) (.Type (Utilities|Struct|BreakDialogGraphPartStructrue _array_element_2)) "NewEnumerator2")
          (LocalVariables|SetSelectionString (Utilities|String|Append (LocalVariables|GetSelectionString) (.Content (Utilities|Struct|BreakDialogGraphPartStructrue _array_element_2))))))
      (Default|AddDialogSelections (Variables|Talk|GetWedgetDialog) (LocalVariables|GetSelectionString)))
    (elif (Utilities|Array|IsValidIndex (.craphchild (Utilities|Array|Get(acopy) (.dialogcontent (Variables|Talk|GetCurrentDialog)) (Variables|Talk|GetDialogIndex))))
      (Variables|Talk|SetDialogIndex (Utilities|Array|Get(acopy) (.craphchild (Utilities|Array|Get(acopy) (.dialogcontent (Variables|Talk|GetCurrentDialog)) (Variables|Talk|GetDialogIndex)))))
      (else
        (Talk|EndDialog)))))

(fn CheckQuestExist
  (params (Quest :type BP%20Quset%20Object%20Reference))
  (return (Utilities|Array|ContainsItem (Variables|Talk|GetQuests) Quest)))