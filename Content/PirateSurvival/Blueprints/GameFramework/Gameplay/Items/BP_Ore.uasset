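; BP_Ore is a mineable rock that breaks apart in stages and drops loot as tools damage it.
; ToolDamage passes health to Damaged, which rounds it up to quarters and cascades through Destruct calls for every stage reached.
; Destruct skips already removed meshes, otherwise swapping the piece for a physics destructible on a short-lived empty Actor (for easy cleanup) and spawning two BP_LootableItem pickups.
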(event EventToolDamage
  (params (HpLeft :type Float%20%28single-precision%29) (TotalHp :type Float%20%28single-precision%29))
  (CallFunction|Damaged HpLeft TotalHp))

(fn ConstructionScript)

(fn Damaged
  (params (Hp :type Float%20%28single-precision%29) (MaxHp :type Float%20%28single-precision%29))
  (switch int (Math|Float|Ceil (/ (/ Hp MaxHp) 0.25))
    (:0
      (CallFunction|Destruct "/Game/EasySurvivalRPG/Meshes/Interactable/Destructable/DM_Rock_Mining_001_4.DM_Rock_Mining_001_4" (Variables|Default|GetSM_Rock_Mining_001_4))
      (CallFunction|Destruct "/Game/EasySurvivalRPG/Meshes/Interactable/Destructable/DM_Rock_Mining_001_3.DM_Rock_Mining_001_3" (Variables|Default|GetSM_Rock_Mining_001_3) :!label _label)
      (CallFunction|Destruct "/Game/EasySurvivalRPG/Meshes/Interactable/Destructable/DM_Rock_Mining_001_2.DM_Rock_Mining_001_2" (Variables|Default|GetSM_Rock_Mining_001_2) :!label _label_2))
    (:1
      (goto _label))
    (:2
      (goto _label_2))
    (:3
      _))
  (CallFunction|Destruct "/Game/EasySurvivalRPG/Meshes/Interactable/Destructable/DM_Rock_Mining_001_1.DM_Rock_Mining_001_1" (Variables|Default|GetSM_Rock_Mining_001_1)))

(fn Destruct
  (params (Destructible :type Destructible%20Mesh%20Object%20Reference) (SM :type Static%20Mesh%20Component%20Object%20Reference))
  (if (and (Utilities|IsValid SM) (Utilities|IsValid Destructible))
    (Components|DestroyComponent SM)
    (bind _returnvalue (Game|SpawnActorfromClass "/Script/Engine.Actor" (Math|Transform|MakeTransform "0, 0, 0" "0, 0, 0" "1,1,1") "Undefined" 0 0)) ; Actor 有一个很好用的属性 life span ,因此搞成Actor可以方便销毁
    (Actor|SetLifeSpan _returnvalue 2.0)
    (bind _returnvalue_2 (AddComponent|AddDestructibleComponent _returnvalue false (Transformation|GetWorldTransform (Variables|Default|GetSM_Rock_Mining_001_5)))) ; 加在生成的空的Actor的身上
    (Class|DestructibleComponent|SetDestructibleMesh _returnvalue_2 Destructible)
    (Collision|SetCollisionResponsetoChannel _returnvalue_2 "ECC_Pawn" "ECR_Ignore")
    (Physics|SetSimulatePhysics _returnvalue_2 true)
    (bind _returnvalue_3 (Game|SpawnActorfromClass "/Game/PirateSurvival/Blueprints/GameFramework/Gameplay/Items/BP_LootableItem.BP_LootableItem_C" (Transformation|GetWorldTransform (Variables|Default|GetSM_Rock_Mining_001_5)) "Undefined" 0 0))
    (Class|LootableItem|SpawnItembyRowNameandCount _returnvalue_3 "10004" 10)
    (bind _returnvalue_4 (Game|SpawnActorfromClass "/Game/PirateSurvival/Blueprints/GameFramework/Gameplay/Items/BP_LootableItem.BP_LootableItem_C" (Transformation|GetWorldTransform (Variables|Default|GetSM_Rock_Mining_001_5)) "AlwaysSpawn" 0 0))
    (Class|LootableItem|SpawnItembyRowNameandCount _returnvalue_4 "10005" 10)))