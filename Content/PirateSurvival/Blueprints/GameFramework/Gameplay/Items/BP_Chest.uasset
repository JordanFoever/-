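; Lootable chest actor for the pirate survival game, seeded with two item types at BeginPlay and exposing its inventory to the interacting player.
; Interacting opens the game HUD and sends every slot in a payload through the pawn's tagged delegate message component to WBP_LootItemBox.
; Inventory changes resend only the changed slot on the same tag.
; Ending interaction collapses the widget; several interface getters are empty stubs.
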(event OnInventoryUpdated(BP_InventoryComponent)
  (params (Index :type Integer))
  (Variables|Default|GetController
    (:then
      (bind _returnvalue (Game|ConstructObjectfromClass "/Game/PirateSurvival/Blueprints/DelegatePayload/BP_LootItemBoxPayload.BP_LootItemBoxPayload_C" self false (Utilities|Map|MakeMap Index (.OutData (Class|InventoryComponent|GetItemData (Variables|Default|GetBP_InventoryComponent) Index)))))
      (bind _returnvalue_2 (Class|AssociatedComponentGetter|GetDelegateComponent(Message) (Pawn|GetControlledPawn (Variables|Default|GetController))))
      (Utilities|IsValid _returnvalue_2
        (:Is%20Valid
          (Class|DelegateComponent|CallDelegate _returnvalue_2 "(TagName=\"GlobalEvent.Interactive.UpdateLootBox\")" _returnvalue) ; 绑定在WBP_LootItemBox中的Construct中
        )))
    (:else)))

(event EventInteractiveResponse
  (params (Controller :type Player%20Controller%20Object%20Reference))
  (CallFunction|HandleInteractiveResponse Controller)
  (Variables|Default|SetController Controller))

(event EventBeginPlay
  (Class|InventoryComponent|AddItemtoInventory (Variables|Default|GetBP_InventoryComponent) "10001" 5 0 0 false)
  (Class|InventoryComponent|AddItemtoInventory (Variables|Default|GetBP_InventoryComponent) "10003" 6 0 0 false))

(event EventEndInteractive
  (params (Controller :type Player%20Controller%20Object%20Reference))
  (bind _asbp_pirate_game_player_controller (Utilities|Casting|CastToBP_PirateGamePlayerController Controller))
  (Widget|SetVisibility (Variables|/Game/PirateSurvival/UI/Game/WBP_GameHUD.WBP_GameHUD_C|GetWBP_LootItemBox (Variables|/Game/PirateSurvival/Blueprints/GameFramework/Gameplay/BP_PirateGamePlayerController.BP_PirateGamePlayerController_C|GetGameHUD _asbp_pirate_game_player_controller)) "Collapsed")
  (Variables|Default|SetOpened false))

(fn ConstructionScript)

(fn HandleInteractiveResponse
  (params (Controller :type Player%20Controller%20Object%20Reference))
  (Variables|Default|SetOpened true)
  (bind _asbp_pirate_game_player_controller (Utilities|Casting|CastToBP_PirateGamePlayerController Controller))
  (Default|SetOpenGameHUD _asbp_pirate_game_player_controller true)
  (bind _returnvalue (Class|AssociatedComponentGetter|GetDelegateComponent(Message) (Pawn|GetControlledPawn Controller)))
  (bind _output_get (LocalVariables|SetDelegateComp _returnvalue))
  (Utilities|IsValid _output_get
    (:Is%20Valid
      (Utilities|FlowControl|Sequence
        (:then_0
          (for _index (range 0 (- (Class|InventoryComponent|GetCapacity (Variables|Default|GetBP_InventoryComponent)) 1))
            (Utilities|Map|Add (LocalVariables|GetDataMap) _index (.OutData (Class|InventoryComponent|GetItemData (Variables|Default|GetBP_InventoryComponent) _index)))))
        (:then_1
          (bind _returnvalue_2 (Game|ConstructObjectfromClass "/Game/PirateSurvival/Blueprints/DelegatePayload/BP_LootItemBoxPayload.BP_LootItemBoxPayload_C" self true (LocalVariables|GetDataMap)))
          (bind _output_get_2 (LocalVariables|SetPayload _returnvalue_2))
          (Class|DelegateComponent|CallDelegate (LocalVariables|GetDelegateComp) "(TagName=\"GlobalEvent.Interactive.UpdateLootBox\")" _output_get_2) ; 绑定委托在WBP_LootItemBox中的 Event Construct 函数中
        )))))

(fn GetPlayerInventoryCapacity
  (return 0))

(fn GetLootableChestInventory
  (return 0))

(fn GetItemData
  (params (Index :type Integer))
  (return (.OutData (Class|InventoryComponent|GetItemData (Variables|Default|GetBP_InventoryComponent) Index))))

(fn GetCraftingComponent
  (return 0))

(fn GetDelegateComponent
  (return 0))

(fn GetHotBarComponent
  (return 0))

(fn GetInteractiveInformation
  (return "" "" "" false))

(fn GetInventoryComponent
  (return (Variables|Default|GetBP_InventoryComponent)))

(fn IsOpen
  (return (Variables|Default|GetOpened)))