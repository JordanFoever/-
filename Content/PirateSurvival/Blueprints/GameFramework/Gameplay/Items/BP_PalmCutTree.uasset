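; BP_PalmCutTree is a damageable palm tree that drops a lootable item when its health runs out.
; AnyDamage feeds a Damage function that subtracts from CurrentHp and, at zero or below, swaps the mesh to a cut palm.
; It spawns a BP_LootableItem at the mesh transform, fills it by row name and count, and enables physics while ignoring WorldDynamic.
; The IsSpawn flag limits the drop to once.
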(event Game|Damage|EventAnyDamage
  (params (Damage :type Float%20%28single-precision%29) (DamageType :type Damage%20Type%20Object%20Reference) (InstigatedBy :type Controller%20Object%20Reference) (DamageCauser :type Actor%20Object%20Reference))
  (CallFunction|Damage Damage))

(fn ConstructionScript)

(fn Damage
  (params (Damage :type Float%20%28single-precision%29))
  (Variables|Default|SetCurrentHp (- (Variables|Default|GetCurrentHp) Damage))
  (if (and (<= (Variables|Default|GetCurrentHp) 0.0) (not (Variables|Default|GetIsSpawn)))
    (Components|StaticMesh|SetStaticMesh (Variables|Default|GetSM_Palm_001) "/Game/EasySurvivalRPG/Meshes/Interactable/SM_Palm_Cut_001.SM_Palm_Cut_001")
    (bind _returnvalue (Game|SpawnActorfromClass "/Game/PirateSurvival/Blueprints/GameFramework/Gameplay/Items/BP_LootableItem.BP_LootableItem_C" (Transformation|GetWorldTransform (Variables|Default|GetSM_Palm_001)) "AlwaysSpawn" 0 0))
    (Class|LootableItem|SpawnItembyRowNameandCount _returnvalue "40001" 5)
    (Collision|SetCollisionEnabled (Variables|/Script/EasySurvivalRPGv2_5.LootableItem|GetStaticMeshComp _returnvalue) "QueryAndPhysics")
    (Collision|SetCollisionResponsetoChannel (Variables|/Script/EasySurvivalRPGv2_5.LootableItem|GetStaticMeshComp _returnvalue) "ECC_WorldDynamic" "ECR_Ignore")
    (Physics|SetSimulatePhysics (Variables|/Script/EasySurvivalRPGv2_5.LootableItem|GetStaticMeshComp _returnvalue) true)
    (Variables|Default|SetIsSpawn true)))