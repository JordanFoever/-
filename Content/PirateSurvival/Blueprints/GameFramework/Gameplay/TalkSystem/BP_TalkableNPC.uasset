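; BP_TalkableNPC is an interactable NPC in the talk system that turns to face whoever is interacting with it.
; Begin and end interaction events store and clear the controller's pawn as the Interactor.
; Tick smoothly interpolates toward a yaw-only look-at rotation, or back to OrginRotation when no Interactor is valid.
; The interaction response is only a debug print, with no dialogue logic here.
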(event EventTick
  (params (DeltaSeconds :type Float%20%28single-precision%29))
  (Variables|Default|SetDelta%20Seconds DeltaSeconds)
  (Utilities|FlowControl|Sequence
    (:then_0
      (bind _interactor (Variables|Default|GetInteractor)
        (:then
          (Variables|Default|SetFacingRotation (Math|Rotator|MakeRotator 0.0 0.0 (.yaw (Math|Rotator|FindLookatRotation (Transformation|GetActorLocation) (Transformation|GetActorLocation _interactor))))))
        (:else
          (Variables|Default|SetFacingRotation (Variables|Default|GetOrginRotation)))))
    (:then_1
      (Transformation|SetActorRotation (Math|Interpolation|RInterpTo (Transformation|GetActorRotation) (Variables|Default|GetFacingRotation) (Variables|Default|GetDelta%20Seconds) 0.0)))))

(event EventEndInteractive
  (params (Controller :type Player%20Controller%20Object%20Reference))
  (Variables|Default|SetInteractor 0))

(event EventBeginInteractive
  (params (Controller :type Player%20Controller%20Object%20Reference))
  (Variables|Default|SetInteractor (Pawn|GetControlledPawn Controller)))

(event EventInteractiveResponse
  (params (Controller :type Player%20Controller%20Object%20Reference))
  (Development|PrintString "Interact"))

(fn ConstructionScript)