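; Player character for the pirate survival game, hosting inventory, hotbar, crafting and building components.
; Component updates reach the HUD as tagged Delegate events with payload objects, and bound crafting UI events return through the same Delegate.
; Input drives building placement, rotation and hold-to-open radial menus for wood, stone and placeables.
; It also saves inventory and buildings to JSON and derives stance from the selected hotbar item's data table row.
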(event OnInventoryUpdated(BP_InventoryComponent)
  (params (Index :type Integer))
  ;[1 1 1] 通知UI更新背包中道具展示的变化
  (bind _returnvalue (Game|ConstructObjectfromClass "/Game/PirateSurvival/Blueprints/DelegatePayload/BP_InventoryIndexPayload.BP_InventoryIndexPayload_C" self Index))
  (Class|DelegateComponent|CallDelegate (Variables|Default|GetDelegate) "(TagName=\"GlobalEvent.PlayerInventory.UpdateSlot\")" _returnvalue) ; 委托的绑定在 GameHUD 中
)

(event OnCraftingListUpdated(Crafting)
  (Class|DelegateComponent|CallDelegate (Variables|Default|GetDelegate) "(TagName=\"GlobalEvent.Crafting.UpdateCraftingList\")") ; 绑定委托在 WBP_GameHUD 中的
)

(event OnInventoryUpdated(BP_HotBarItemComponent)
  (params (Index :type Integer))
  (bind _returnvalue (Game|ConstructObjectfromClass "/Game/PirateSurvival/Blueprints/DelegatePayload/BP_InventoryIndexPayload.BP_InventoryIndexPayload_C" self Index))
  (Class|DelegateComponent|CallDelegate (Variables|Default|GetDelegate) "(TagName=\"GlobalEvent.HotBar.UpdateSlot\")" _returnvalue) ; 委托的绑定在 GameHUD 中
)

(event OnstartCrafting(Crafting)
  (Class|DelegateComponent|CallDelegate (Variables|Default|GetDelegate) "(TagName=\"GlobalEvent.Crafting.StartCrafting\")"))

(event OnShowBuildingWarnandTipInfo(BP_BuildingSystemComponent)
  (params (InfoDescription :type Name :default "None") (IsTip :type Boolean) (IsShowCanBuilding :type Boolean))
  ;[1 1 1] 打开建造面板选择建造部件时选择以及建造时的提示信息
  (bind _returnvalue (Game|ConstructObjectfromClass "/Game/PirateSurvival/Blueprints/DelegatePayload/BP_BuildingTipInfoPayload.BP_BuildingTipInfoPayload_C" self InfoDescription IsTip IsShowCanBuilding))
  (Class|DelegateComponent|CallDelegate (Variables|Default|GetDelegate) "(TagName=\"GlobalEvent.BuildingSystem.ShowBuildingTipInformation\")" _returnvalue))

(event EventOnGameUIInitiated
  (Class|InventoryComponent|PostInventoryInitiate (Variables|Default|GetBP_InventoryComponent))
  (Class|CraftingComponent|PostInitiateList (Variables|Default|GetCrafting)))

(event EventHotBarSelected
  (params (HotBarComp :type Inventory%20Component%20Object%20Reference) (Index :type Integer))
  (bind _asbp_hot_bar_item_component (Utilities|Casting|CastToBP_HotBarItemComponent HotBarComp))
  (Default|Select _asbp_hot_bar_item_component Index))

(event EventNotifyPlayerSaveLevelData
  (params (IsSaveData :type Boolean))
  (Utilities|FlowControl|Sequence
    (:then_0
      (if IsSaveData
        (Class|InventoryComponent|SaveDatatoJsonFile (Variables|Default|GetBP_InventoryComponent))
        (Class|BuildingSystemComponent|SaveDatatoJsonFile (Variables|Default|GetBP_BuildingSystemComponent))))
    (:then_1
      (Default|SetOpenSaveConfirmUI (.AsBP%20Pirate%20Game%20Player%20Controller (Utilities|Casting|CastToBP_PirateGamePlayerController (Game|GetPlayerController 0))) false))))

(event EventToggleBuildingPart
  (params (Index :type Integer))
  ;[1 1 1] 切换建造部件
  (Class|BuildingSystemComponent|ToggleBuildingPart (Variables|Default|GetBP_BuildingSystemComponent) Index))

(event Input|MouseEvents|MouseWheelAxis
  (params (AxisValue :type Float%20%28single-precision%29))
  (Class|BuildingSystemComponent|RotateBuildingPart (Variables|Default|GetBP_BuildingSystemComponent) AxisValue))

(event Input|MouseEvents|LeftMouseButton
  (params (Key :type Key%20Structure :default "None")))

(event Input|KeyboardEvents|Q
  (params (Key :type Key%20Structure :default "None"))
  ;[1 1 1] 打开建造菜单
  (:Pressed
    (Building|OpenCircleBuildingMenu "WoodBuildingMenu"))
  (:Released
    (Building|CloseCircleBuildingMenu "WoodBuildingMenu")))

(event Input|KeyboardEvents|T
  (params (Key :type Key%20Structure :default "None"))
  ;[1 1 1] 打开建造菜单
  (:Pressed
    (Building|OpenCircleBuildingMenu "PlaceableBuildingMenu"))
  (:Released
    (Building|CloseCircleBuildingMenu "PlaceableBuildingMenu")))

(event Input|KeyboardEvents|G
  (params (Key :type Key%20Structure :default "None"))
  ;[1 1 1] 打开建造菜单
  (:Pressed
    (Building|OpenCircleBuildingMenu "StoneBuildingMenu"))
  (:Released
    (Building|CloseCircleBuildingMenu "StoneBuildingMenu")))

(event Input|KeyboardEvents|E
  (params (Key :type Key%20Structure :default "None"))
  (:Pressed
    (if (Class|BuildingSystemComponent|CanStartBuild (Variables|Default|GetBP_BuildingSystemComponent))
      (Class|BuildingSystemComponent|PlaceBuildingPart (Variables|Default|GetBP_BuildingSystemComponent)))))

(fn ConstructionScript
  (Class|DelegateComponent|BindDelegate (Variables|Default|GetDelegate) "(TagName=\"GlobalEvent.Crafting.UISelectCagetory\")" self "HandleCraftingCategory")
  (bind _outrownames (DataTable|GetDataTableRowNames "/Game/PirateSurvival/DataTables/Table_CraftingInfo.Table_CraftingInfo"))
  (Variables|/Script/EasySurvivalRPGv2_5.CraftingComponent|SetCraftingInfoList (Variables|Default|GetCrafting) _outrownames)
  (Class|DelegateComponent|BindDelegate (Variables|Default|GetDelegate) "(TagName=\"GlobalEvent.Crafting.UISelectCraftingItem\")" self "HandleUISelectCraftingItem")
  (Class|DelegateComponent|BindDelegate (Variables|Default|GetDelegate) "(TagName=\"GlobalEvent.Crafting.UIStartCrafting\")" self "HandleUIStartCrafting"))

(fn GetInventoryComponent
  (return (Variables|Default|GetBP_InventoryComponent)))

(fn GetDelegateComponent
  (return (Variables|Default|GetDelegate)))

(fn GetHotBarComponent
  (return (Variables|Default|GetBP_HotBarItemComponent)))

(fn HandleCraftingCategory
  (params (Payload :type Object%20Object%20Reference))
  (bind _asbp_inventory_index_payload (Utilities|Casting|CastToBP_InventoryIndexPayload Payload))
  (Class|CraftingComponent|SetCraftingCategory (Variables|Default|GetCrafting) (Utilities|Array|Get(acopy) (Utilities|Array|MakeArray "All" "Equipment" "Component" "Building" "Consumable" "Weapon" "Ammo" "Tool") (Variables|/Game/PirateSurvival/Blueprints/DelegatePayload/BP_InventoryIndexPayload.BP_InventoryIndexPayload_C|GetIndex _asbp_inventory_index_payload))))

(fn HandleUISelectCraftingItem
  (params (Payload :type Object%20Object%20Reference))
  (bind _asbp_inventory_index_payload (Utilities|Casting|CastToBP_InventoryIndexPayload Payload))
  (Class|DelegateComponent|CallDelegate (Variables|Default|GetDelegate) "(TagName=\"GlobalEvent.Crafting.UpdateCraftingInfo\")" _asbp_inventory_index_payload)
  (Class|CraftingComponent|SelectCraftingItem (Variables|Default|GetCrafting) (Variables|/Game/PirateSurvival/Blueprints/DelegatePayload/BP_InventoryIndexPayload.BP_InventoryIndexPayload_C|GetIndex _asbp_inventory_index_payload)))

(fn HandleUIStartCrafting
  (params (Payload :type Object%20Object%20Reference))
  (bind _asbp_inventory_index_payload (Utilities|Casting|CastToBP_InventoryIndexPayload Payload))
  (Class|CraftingComponent|StartCrafting (Variables|Default|GetCrafting) (Variables|/Game/PirateSurvival/Blueprints/DelegatePayload/BP_InventoryIndexPayload.BP_InventoryIndexPayload_C|GetIndex _asbp_inventory_index_payload)))

(fn GetCameraProjectData
  (return (Transformation|GetWorldLocation (Variables|Default|GetSpringArm)) (Pawn|GetControlRotation :!class /Script/Engine.Pawn)))

(fn OpenCircleBuildingMenu
  (params (MenuType :type ECircleBuildingMenuType%20Enum :default "WoodBuildingMenu"))
  (LocalVariables|SetBuildingMenuType MenuType)
  (Variables|/Script/EasySurvivalRPGv2_5.BuildingSystemComponent|SetCurrentOpenCircleMenuType (Variables|Default|GetBP_BuildingSystemComponent) (LocalVariables|GetBuildingMenuType))
  (Class|BuildingSystemComponent|CancelBuilding (Variables|Default|GetBP_BuildingSystemComponent))
  (Variables|/Script/Engine.PlayerController|SetbShowMouseCursor (Game|GetPlayerController 0) true)
  (Input|SetInputModeGameandUI (Game|GetPlayerController 0) 0 "DoNotLock" true)
  (bind _returnvalue (Game|ConstructObjectfromClass "/Game/PirateSurvival/Blueprints/DelegatePayload/BP_BuildingMenuTypePayload.BP_BuildingMenuTypePayload_C" self (LocalVariables|GetBuildingMenuType) true))
  (Class|DelegateComponent|CallDelegate (Variables|Default|GetDelegate) "(TagName=\"GlobalEvent.BuildingSystem.OpenAndCloseBuildingMenu\")" _returnvalue))

(fn CloseCircleBuildingMenu
  (params (MenuType :type ECircleBuildingMenuType%20Enum :default "WoodBuildingMenu"))
  (LocalVariables|SetBuildingMenuType MenuType)
  (Variables|/Script/Engine.PlayerController|SetbShowMouseCursor (Game|GetPlayerController 0) false)
  (Input|SetInputModeGameOnly (Game|GetPlayerController 0))
  (bind _returnvalue (Game|ConstructObjectfromClass "/Game/PirateSurvival/Blueprints/DelegatePayload/BP_BuildingMenuTypePayload.BP_BuildingMenuTypePayload_C" self (LocalVariables|GetBuildingMenuType)))
  (Class|DelegateComponent|CallDelegate (Variables|Default|GetDelegate) "(TagName=\"GlobalEvent.BuildingSystem.OpenAndCloseBuildingMenu\")" _returnvalue))

(fn GetCraftingList
  (bind _crafting (Variables|Default|GetCrafting))
  (return (Class|CraftingComponent|GetCraftingCategory _crafting) (Class|CraftingComponent|GetCurrentCraftingList _crafting)))

(fn GetCraftingListQueueLength
  (return 0))

(fn GetHotBarItemData
  (params (Index :type Integer))
  (return (.OutData (Class|InventoryComponent|GetItemData (Variables|Default|GetBP_HotBarItemComponent) Index))))

(fn GetItemData
  (params (Index :type Integer))
  (return (.OutData (Class|InventoryComponent|GetItemData (Variables|Default|GetBP_InventoryComponent) Index))))

(fn GetPlayerInventoryCapacity
  (return (Class|InventoryComponent|GetCapacity (Variables|Default|GetBP_InventoryComponent))))

(fn GetPlayerStance
  (bind _returnvalue (Utilities|GetDataTableRow "/Game/PirateSurvival/DataTables/Table_WeaponAndTools.Table_WeaponAndTools" (.tablerowname (Default|GetSelectedItemData (Variables|Default|GetBP_HotBarItemComponent))))
    (:then
      (return (.stancetype _returnvalue)))
    (:RowNotFound
      (return "Common"))))

(fn GetProcessingCraftingData
  (params (Index :type Integer))
  (return "None" 0 false))