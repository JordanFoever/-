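; Hotbar item component that tracks which slot of the owner's hotbar is currently selected in the survival game.
; Select validates a new index against capacity, stores it and returns that slot's item data, while GetSelectedItemData reads the current one.
; Selection changes go through the owner's delegate message component as a tagged event with an index payload object, which a comment notes WBP_GameHUD binds.
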(fn Select
  (params (Index :type Integer))
  (if (Math|Boolean|ANDBoolean (>= Index 0) (< Index (Class|InventoryComponent|GetCapacity)) (!= Index (Variables|Default|GetCurrentIndex)))
    (Variables|Default|SetCurrentIndex Index)
    (bind _returnvalue (Class|AssociatedComponentGetter|GetDelegateComponent(Message) (Components|GetOwner)))
    (bind _returnvalue_2 (Game|ConstructObjectfromClass "/Game/PirateSurvival/Blueprints/DelegatePayload/BP_InventoryIndexPayload.BP_InventoryIndexPayload_C" self (Variables|Default|GetCurrentIndex)))
    (Class|DelegateComponent|CallDelegate _returnvalue "(TagName=\"GlobalEvent.HotBar.UpdateSelection\")" _returnvalue_2) ; 绑定委托在WBP_GameHUD
    (return (.OutData (Class|InventoryComponent|GetItemData Index)))))

(fn GetSelectedItemData
  (return (.OutData (Class|InventoryComponent|GetItemData (Variables|Default|GetCurrentIndex)))))