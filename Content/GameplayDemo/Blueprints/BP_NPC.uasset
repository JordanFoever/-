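; BP_NPC is an interactable quest-giver NPC that shows a talk prompt and holds conversations with the player.
; While interacting, it smoothly yaws toward the player's pawn each tick, then turns back to its original rotation afterward.
; On interaction it sends the controller default, quest-complete or quest-incomplete dialog, depending on its current quest's state.
; Choosing the first dialog reply creates a BP_FindingItemQuest and passes it to the player's controller.
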(event EventInteractiveResponse
  (params (Controller :type Player%20Controller%20Object%20Reference))
  (bind _exist (Class|BPIDialogListener|CheckQuestExist(Message) Controller (Variables|Default|GetCurrentProssessQuest)))
  (if (not _exist)
    (Class|BPIDialogListener|ListenDialog(Message) Controller (Variables|Default|GetDialog%20Content))
    (elif (Default|CheckAccomlished (Variables|Default|GetCurrentProssessQuest))
      (Class|BPIDialogListener|ListenDialog(Message) Controller (Variables|Default|GetDialogQuestComplete))
      (else
        (Class|BPIDialogListener|ListenDialog(Message) Controller (Variables|Default|GetDialogQuestUnComplete))))))

(event EventBeginInteractive
  (params (Controller :type Player%20Controller%20Object%20Reference))
  (Variables|Default|SetInteractor (Pawn|GetControlledPawn Controller)))

(event EventTick
  (params (DeltaSeconds :type Float%20%28single-precision%29))
  (Variables|Default|SetDelta%20Seconds DeltaSeconds)
  (Utilities|FlowControl|Sequence
    (:then_0
      (bind _interactor (Variables|Default|GetInteractor)
        (:then
          (Variables|Default|SetFacingRotation (Math|Rotator|MakeRotator 0.0 0.0 (.yaw (Math|Rotator|FindLookatRotation (Transformation|GetActorLocation) (Transformation|GetActorLocation _interactor))))))
        (:else
          (Variables|Default|SetFacingRotation (Variables|Default|GetOriginRotation)))))
    (:then_1
      (Transformation|SetActorRotation (Math|Interpolation|RInterpTo (Transformation|GetActorRotation) (Variables|Default|GetFacingRotation) (Variables|Default|GetDelta%20Seconds) 8.0)))))

(event EventEndInteractive
  (params (Controller :type Player%20Controller%20Object%20Reference))
  (Variables|Default|SetInteractor 0) ; 设置为空
)

(fn ConstructionScript)

(fn ReplyDialog
  (params (GraphIndex :type Integer) (SelectionIndex :type Integer))
  (switch int SelectionIndex
    (:0
      (bind _returnvalue (Game|ConstructObjectfromClass "/Game/GameplayDemo/Blueprints/Quest/BP_FindingItemQuest.BP_FindingItemQuest_C" (Variables|Default|GetInteractor) 99 (.AsPlayer%20Controller (Utilities|Casting|CastToPlayerController (Pawn|GetController (Variables|Default|GetInteractor))))))
      (bind _output_get (Variables|Default|SetCurrentProssessQuest _returnvalue))
      (Class|BPIDialogListener|ReceiveQuest(Message) (Pawn|GetController (Variables|Default|GetInteractor)) _output_get))))

(fn GetInteractiveInformation
  (return "Name: AAA" "I am a homeless person " "Press \"F\" to Talk" true))