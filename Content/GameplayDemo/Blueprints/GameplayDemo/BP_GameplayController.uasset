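; Player controller that handles actor interaction, branching NPC dialogue and a list of received quests.
; Each tick a box trace ahead of the pawn tracks BPI_InteractiveActor targets with begin/end messages, and F interacts with the current one.
; Dialogue is walked as an indexed graph through WBP_DialogPannel, showing choices at branches and reporting picks to the NPC.
; It switches input mode and mouse capture around conversations.
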(event EventBeginPlay
  (bind _returnvalue (UserInterface|CreateWidget "/Game/GameplayDemo/Blueprints/UI/WBP_DialogPannel.WBP_DialogPannel_C"))
  (bind _output_get (Variables|Default|SetWedgetDialog _returnvalue))
  (Widget|SetVisibility _output_get "Collapsed") ; 折叠状态不占有空间
  (UserInterface|Viewport|AddtoViewport (Variables|Default|GetWedgetDialog) 0))

(event EventTick
  (params (DeltaSeconds :type Float%20%28single-precision%29))
  (CallFunction|UpdateInteractiveTrace))

(event EventListenDialog
  (params (DialogContent :type Dialog%20Structure%20Structure))
  (Variables|Default|SetCurrentDialog DialogContent)
  (Widget|SetVisibility (Variables|Default|GetWedgetDialog) "Visible")
  (Input|SetInputModeGameandUI self (Variables|Default|GetWedgetDialog) "DoNotLock" true)
  (Variables|Default|SetbShowMouseCursor true)
  (Class|GameplayStatics|SetViewportMouseCaptureMode "NoCapture")
  (Variables|Default|SetProssessingDialog true)
  (Variables|Default|SetCurrentDialogNPC (.AsBP%20NPC (Utilities|Casting|CastToBP_NPC (Variables|Default|GetCurrentInteractiveActor))))
  (CallFunction|ProssessDialog))

(event EventContinueDialog
  (CallFunction|ProssessDialog))

(event EventFinishDialogGraph
  (CallFunction|HandleFinishDialogGraph))

(event EventHandleDialogSelected
  (params (Index :type Integer))
  (Default|ReplyDialog (Variables|Default|GetCurrentDialogNPC) (Variables|Default|GetDialogIndex) Index)
  (Variables|Default|SetDialogIndex (Utilities|Array|Get(acopy) (.craphchild (Utilities|Array|Get(acopy) (.dialogcontent (Variables|Default|GetCurrentDialog)) (Variables|Default|GetDialogIndex))) Index))
  (CallFunction|ProssessDialog))

(event EventQuest
  (params (Quest :type BP%20Quset%20Object%20Reference))
  (Utilities|Array|Add (Variables|Default|GetQuests) Quest))

(event Input|KeyboardEvents|F
  (params (Key :type Key%20Structure :default "None"))
  (:Pressed
    (bind _currentinteractiveactor (Variables|Default|GetCurrentInteractiveActor) ; 判断当前交互的对象是否是Actor，并且当前交互的Actor必须只能是NPC
      (:then
        (Class|BPIInteractiveActor|Interacted(Message) _currentinteractiveactor (Pawn|GetControlledPawn)))
      (:else))))

(fn ConstructionScript)

(fn UpdateInteractiveTrace
  (bind _returnvalue (Pawn|GetControlledPawn))
  (bind _returnvalue_2 (Pawn|GetControlledPawn))
  (bind _interactiveoffset (Variables|Default|GetInteractiveOffset))
  (bind _returnvalue_3 (Transformation|GetActorTransform _returnvalue))
  (bind _returnvalue_4 (Math|Transform|TransformLocation _returnvalue_3 _interactiveoffset))
  (bind (_outhit _returnvalue_5) (Collision|BoxTraceByChannel (+ _returnvalue_4 (Math|Vector|MakeVector 0.0 0.0 (Variables|Default|GetInteractiveTraceRange))) (- _returnvalue_4 (Math|Vector|MakeVector 0.0 0.0 (Variables|Default|GetInteractiveTraceRange))) "50.000000,50.000000, 0" (Transformation|GetActorRotation _returnvalue_2) "TraceTypeQuery1" false (Utilities|Array|MakeArray _returnvalue_2) "ForOneFrame"))
  (Utilities|FlowControl|Sequence
    (:then_0
      (bind _output_get (LocalVariables|SetTraceInteractiveActor (.HitActor (Collision|BreakHitResult _outhit))))
      (if (and _returnvalue_5 (Utilities|DoesObjectImplementInterface _output_get "/Game/GameplayDemo/Blueprints/Interfaces/BPI_InteractiveActor.BPI_InteractiveActor_C"))
        (if (!= (Variables|Default|GetCurrentInteractiveActor) (LocalVariables|GetTraceInteractiveActor))
          (Class|BPIInteractiveActor|BeginInteractive(Message) (LocalVariables|GetTraceInteractiveActor) (Pawn|GetControlledPawn))
          (bind _currentinteractiveactor (Variables|Default|GetCurrentInteractiveActor :!label _label) ; 之前交互到离开交互状态
            (:then
              (Class|BPIInteractiveActor|EndInteractive(Message) _currentinteractiveactor))
            (:else)))
        (else
          (goto _label))))
    (:then_1
      (Variables|Default|SetCurrentInteractiveActor (LocalVariables|GetTraceInteractiveActor)))))

(fn ProssessDialog
  ;[1 1 1] 如果继续进行对话就获取这个对话中的一段从第一段开始并将这对话的内容 传给  add dialog Draph（DialogGraphStructure[ ]   DialogGraph）
  (if (Variables|Default|GetProssessingDialog)
    (if (Utilities|Array|IsValidIndex (.dialogcontent (Variables|Default|GetCurrentDialog)) (Variables|Default|GetDialogIndex))
      (Default|AddDialogGraph (Variables|Default|GetWedgetDialog) (.graph (Utilities|Array|Get(acopy) (.dialogcontent (Variables|Default|GetCurrentDialog)) (Variables|Default|GetDialogIndex)))))
    (else
      ;[1 1 1] 这个是结束对话时调用
      (Input|SetInputModeGameOnly self)
      (Variables|Default|SetbShowMouseCursor false)
      (Widget|SetVisibility (Variables|Default|GetWedgetDialog) "Collapsed")
      (Class|GameplayStatics|SetViewportMouseCaptureMode "CapturePermanently") ; 永久捕获鼠标
      (Widget|Panel|ClearChildren (Variables|/Game/GameplayDemo/Blueprints/UI/WBP_DialogPannel.WBP_DialogPannel_C|GetScrollBox_DialogContainer (Variables|Default|GetWedgetDialog))))))

(fn HandleFinishDialogGraph
  (if (> (Utilities|Array|Length (.craphchild (Utilities|Array|Get(acopy) (.dialogcontent (Variables|Default|GetCurrentDialog)) (Variables|Default|GetDialogIndex)))) 1) ; 为true右分支，反之没有继续执行对话
    (for (_array_element _array_index) (.craphchild (Utilities|Array|Get(acopy) (.dialogcontent (Variables|Default|GetCurrentDialog)) (Variables|Default|GetDialogIndex)))
      (LocalVariables|SetSelectionString (Utilities|String|Append (Utilities|String|ToString(Integer) (+ _array_index 1)) ". "))
      (for _array_element_2 (.graph (Utilities|Array|Get(acopy) (.dialogcontent (Variables|Default|GetCurrentDialog)) _array_element))
        (if (Utilities|Enum|Equal(Enum) (.Type (Utilities|Struct|BreakDialogGraphPartStructrue _array_element_2)) "NewEnumerator2")
          (LocalVariables|SetSelectionString (Utilities|String|Append (LocalVariables|GetSelectionString) (.Content (Utilities|Struct|BreakDialogGraphPartStructrue _array_element_2))))))
      (Default|AddDialogSelections (Variables|Default|GetWedgetDialog) (LocalVariables|GetSelectionString)))
    (elif (Utilities|Array|IsValidIndex (.craphchild (Utilities|Array|Get(acopy) (.dialogcontent (Variables|Default|GetCurrentDialog)) (Variables|Default|GetDialogIndex))))
      (Variables|Default|SetDialogIndex (Utilities|Array|Get(acopy) (.craphchild (Utilities|Array|Get(acopy) (.dialogcontent (Variables|Default|GetCurrentDialog)) (Variables|Default|GetDialogIndex)))))
      (else
        (CallFunction|EndDialog)))))

(fn EndDialog
  (Variables|Default|SetProssessingDialog false)
  (Default|AddEndDialogTip (Variables|Default|GetWedgetDialog))
  (Variables|Default|SetCurrentDialogNPC 0)
  (Variables|Default|SetDialogIndex 0))

(fn CheckQuestExist
  (params (Quest :type BP%20Quset%20Object%20Reference))
  (return (Utilities|Array|ContainsItem (Variables|Default|GetQuests) Quest)))